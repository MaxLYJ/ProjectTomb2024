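; Tutorial room Blueprint that procedurally builds a simple tiled room when play begins.
; CreateRoomTutorial lays a grid of floor instances sized by tile count and tile size, then adds raised instances along the two opposite X edges as walls.
; Both walls share a door gap set by DoorOffset and DoorWidth.
; Floor and walls reuse one instanced static mesh component; HasDoor is unused.
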(event `self.ReceiveBeginPlay`
  (`self.CreateRoom_tutorial`))

(fn `CreateRoom_tutorial`
  (bind _returnvalue (+ (`self.DoorOffset`) 0))
  ;[1 1 1] CreateFloor
  (for _index (range (+ (`self.TileX`) 1))
    (for _index_2 (range (+ (`self.TileY`) 1))
      (`InstancedStaticMeshComponent.AddInstance` (`self.InstancedStaticMesh_Floor`) (`KismetMathLibrary.MakeTransform` (`KismetMathLibrary.MakeVector` (`KismetMathLibrary.Conv_IntToDouble` (* _index (`self.TileSizeX`))) (`KismetMathLibrary.Conv_IntToDouble` (* _index_2 (`self.TileSizeY`))))) false)))
  (for _index_3 (range (+ (`self.TileY`) 1))
    ;[1 1 1] Wall0
    (if (not (and (< _index_3 (+ _returnvalue (`self.DoorWidth`))) (> _index_3 (- _returnvalue 1))))
      (`InstancedStaticMeshComponent.AddInstance` (`self.InstancedStaticMesh_Floor`) (`KismetMathLibrary.MakeTransform` (`KismetMathLibrary.MakeVector` 0.0 (`KismetMathLibrary.Conv_IntToDouble` (* _index_3 (`self.TileSizeY`))) 100.0)) false)
      (`InstancedStaticMeshComponent.AddInstance` (`self.InstancedStaticMesh_Floor`) (`KismetMathLibrary.MakeTransform` (`KismetMathLibrary.MakeVector` (`KismetMathLibrary.Conv_IntToDouble` (* (`self.TileX`) (`self.TileSizeX`))) (`KismetMathLibrary.Conv_IntToDouble` (* _index_3 (`self.TileSizeY`))) 100.0)) false))))

(fn `UserConstructionScript`)