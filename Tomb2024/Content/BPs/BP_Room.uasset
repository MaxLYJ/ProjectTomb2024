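; BP_Room is a room Blueprint that builds a flat rectangular grid of tiles from an instanced static mesh cube.
; CreateRoom runs nested loops over the X and Y tile counts, adding one instance per cell, spaced by tile size at Z zero.
; Both the Construction Script and BeginPlay call CreateRoom, which adds instances without clearing existing ones.
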(event `self.ReceiveBeginPlay`
  (`self.CreateRoom`))

(fn `CreateRoom`
  (for _index (range (`self.RoomTilesY`))
    (for _index_2 (range (`self.RoomTilesX`))
      (`InstancedStaticMeshComponent.AddInstance` (`self.InstancedStaticMesh_Cube`) (`KismetMathLibrary.MakeTransform` (`KismetMathLibrary.MakeVector` (* (`self.TileSizeX`) _index_2) (* _index (`self.TilesSizeY`)))) false)))
  (return))

(fn `UserConstructionScript`
  (`self.CreateRoom`))